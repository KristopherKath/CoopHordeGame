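; BP_Projectile is a projectile actor that explodes on a short timed fuse after it spawns.
; BeginPlay waits out a delay, calls the Explode event, then hides the Sphere component and destroys the actor.
; Explode spawns a particle emitter, applies radial damage credited to the instigating controller, and draws a debug sphere showing the blast radius.
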(event `self.ReceiveBeginPlay`
  (`KismetSystemLibrary.Delay` 1.0)
  (`self.Explode`)
  (`SceneComponent.SetVisibility` (`self.Sphere`) false false)
  (`self.K2_DestroyActor`))

(event `Explode`
  (bind _returnvalue (`self.K2_GetActorLocation`))
  (`GameplayStatics.SpawnEmitterAtLocation` "/Game/WeaponEffects/Explosion/P_Explosion.P_Explosion" _returnvalue)
  (`GameplayStatics.ApplyRadialDamage` :`BaseDamage` 20.0 :`Origin` _returnvalue :`DamageRadius` 200.0 :`DamageCauser` self :`InstigatedByController` (`self.GetInstigatorController`))
  (`KismetSystemLibrary.DrawDebugSphere` _returnvalue 200.0 12 (struct :`R` 1.0 :`G` 0.622348 :`A` 1.0) 1.0))

(fn `UserConstructionScript`)